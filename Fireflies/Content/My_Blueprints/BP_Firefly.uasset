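; BP_Firefly is a firefly actor Blueprint that currently has no working behavior.
; Tick range-checks the truncated frame DeltaSeconds modulo 5, but the branch does nothing.
; A disconnected AddActorLocalTransform node would offset the actor by its own location scaled by negative DeltaSeconds, along with its current rotation and scale, but it never runs.
; The construction script is empty.
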(event EventTick
  (params (DeltaSeconds :type Float%20%28single-precision%29))
  (if (Math|Integer|InRange(Integer) (Math|Integer|%(Integer) (Math|Float|Truncate DeltaSeconds) 5) 0 2)
    _))

(fn ConstructionScript)