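; BP_Stand is a stand actor with a Key1 component and a Sphere that toggles between two states on successive actor overlaps.
; A FlipFlop first shifts Key1 aside, applies an upward impulse to Sphere and sets IsDown.
; The next overlap moves Key1 and Sphere to fixed raised relative positions, leaving IsDown true.
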(event EventBeginPlay)

(event Collision|EventActorBeginOverlap
  (params (OtherActor :type Actor%20Object%20Reference))
  (Utilities|FlowControl|FlipFlop
    (:A
      (Transformation|SetRelativeLocation (Variables|Default|GetKey1) "-90.000000, 0, 0" false false)
      (Physics|AddImpulseatLocation (Variables|Default|GetSphere) (* "0, 0,5.000000" 1e+02) (Transformation|GetActorLocation) "None")
      (Variables|Default|SetisDown true))
    (:B
      (Transformation|SetRelativeLocation (Variables|Default|GetKey1) "0.000000, 0,123.000000" false false)
      (Transformation|SetRelativeLocation (Variables|Default|GetSphere) "0.000000, 0,140.000000" false false))))

(event EventTick
  (params (DeltaSeconds :type Float%20%28single-precision%29)))

(fn ConstructionScript)